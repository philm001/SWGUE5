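; Player character Blueprint that builds its mesh from merged parts and handles sprinting, interaction and the inventory UI.
; On BeginPlay it merges the skeletal meshes, then the local player gets the HUD widget, which toggles inventory view and shows health and hunger.
; Interact traces from the camera, via server call on clients.
; New items spawn off-world actors from Medpack, Armor or Food DataTables, with render targets feeding inventory widgets.
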(event `self.ReceiveBeginPlay`
  (bind _returnvalue (`MeshMergeLibrary.MergeMeshes` (`self.MeshMergeParameters`)))
  (`/Engine/EditorBlueprintResources/StandardMacros.IsValid` _returnvalue
    (:`Is Valid`
      (`SkinnedMeshComponent.SetSkinnedAssetAndUpdate` (`self.Mesh`) _returnvalue true)
      (if (`self.IsLocallyControlled`)
        (bind _returnvalue_2 (`|CreateWidget` "/Game/User_Interfaces/W_UI.W_UI_C"))
        (set `self.W_UI` _returnvalue_2)
        (`UserWidget.AddToViewport` _returnvalue_2 0)))))

(event `Key|I`
  (params (Key :type "Key Structure"))
  (bind _w_ui (`self.W_UI`))
  (:`Pressed`
    (`/Engine/EditorBlueprintResources/StandardMacros.FlipFlop`
      (:`A`
        (`/Game/User_Interfaces/W_UI.DisplayInventory` _w_ui))
      (:`B`
        (`/Game/User_Interfaces/W_UI.DisplayDefaultView` _w_ui)))
    (`AddComponent|NODE_AddAudioComponent-0`)))

(event `self.UpdateStats`
  (params (NewHunger :type "Float (single-precision)") (NewHealth :type "Float (single-precision)"))
  (`/Game/User_Interfaces/W_UI.UpdateStats` (`self.W_UI`) NewHealth NewHunger))

(event `InputAction|Running`
  (params (Key :type "Key Structure"))
  (bind _charactermovement (`self.CharacterMovement`))
  (:`Pressed`
    (set `CharacterMovementComponent.MaxWalkSpeed` 800.0 _charactermovement))
  (:`Released`
    (set `CharacterMovementComponent.MaxWalkSpeed` 225.0 _charactermovement)))

(event `InputAction|Interact`
  (params (Key :type "Key Structure"))
  (bind _camera (`self.Camera`))
  (bind _returnvalue (`SceneComponent.K2_GetComponentLocation` _camera))
  (bind _returnvalue_2 (+ _returnvalue (* (`SceneComponent.GetForwardVector` _camera) 5000.0)))
  (:`Pressed`
    (if (`self.HasAuthority` self)
      (`self.Interact` self _returnvalue _returnvalue_2)
      (else
        (`self.Server_Interact` self _returnvalue _returnvalue_2)))))

(event `self.UpdateInventoryWidget`
  (params (NewInventoryItems :type "Array of ItemData Structure (by ref)")))

(event `self.AddItemandUpdateInventortyWidgetTest`
  (params (ItemStored :type "ItemData Structure") (CurrentInventory :type "Array of ItemData Structure (by ref)"))
  (bind _tempitemdata (`self.TempItemData`))
  (bind _returnvalue (`KismetMathLibrary.Conv_VectorToTransform` (`KismetMathLibrary.MakeVector` -1000.0 -1000.0 -1000.0)))
  (bind _w_inventory (`/Game/User_Interfaces/W_UI.W_Inventory` (`self.W_UI`)))
  (bind _addnewitem (`/Game/User_Interfaces/W_Inventory.ShouldAddNewItem` _w_inventory CurrentInventory))
  (if _addnewitem
    (bind _output_get (set `self.TempItemData` ItemStored))
    (bind (_itemclass _itemcost _internalname _datatablename) (break `ItemData` _output_get))
    (`KismetSystemLibrary.PrintString` _internalname)
    (switch `string` _datatablename
      (:`MedpackDT`
        (bind _returnvalue_2 (`KismetStringLibrary.Conv_StringToName` _internalname))
        (bind _returnvalue_3 (`|GetDataTableRow` "/Game/Blueprints/Struct/MedpackDT.MedpackDT" _returnvalue_2)
          (:`then`
            (bind (_itemid _itembueprintclass _render_target) (break `/Game/Blueprints/Struct/TestStruct` _returnvalue_3))
            (bind _returnvalue_4 (`|SpawnActorFromClass` _itembueprintclass (`KismetMathLibrary.Conv_VectorToTransform` (`KismetMathLibrary.MakeVector` -2000.0 -1000.0 -1000.0)) "Undefined" "OverrideRootScale" null null))
            (`self.SetInventoryItemWidgetStatic` _returnvalue_4 (`self.TempItemData`) _render_target))
          (:`RowNotFound`
            (`KismetSystemLibrary.PrintString` "row DNE"))))
      (:`ArmorDT`
        (bind _returnvalue_5 (`|GetDataTableRow` "/Game/Blueprints/Struct/BoneArmorDT.BoneArmorDT" _returnvalue_2)
          (:`then`
            (bind (_internalname_2 _itemgamename _itemblueprintclass _render_target_2 _skeletalemeshreference) (break `ArmorDTStruct` _returnvalue_5))
            (bind _returnvalue_6 (`|SpawnActorFromClass` _itemblueprintclass _returnvalue "Undefined" "OverrideRootScale" null null))
            (`AnimatedItem.SetSkinnedAssetAndUpdate` _returnvalue_6 _skeletalemeshreference)
            (`self.SetInventoryItemWidgetAnimated` _returnvalue_6 _tempitemdata _render_target_2))))
      (:`FoodDT`
        (bind _returnvalue_7 (`|GetDataTableRow` "/Game/Blueprints/Struct/FoodDT.FoodDT" _returnvalue_2)
          (:`then`
            (bind (_itemid_2 _itembueprintclass_2 _render_target_3) (break `/Game/Blueprints/Struct/FoodStruct` _returnvalue_7))
            (bind _returnvalue_8 (`|SpawnActorFromClass` _itembueprintclass_2 _returnvalue "Undefined" "OverrideRootScale" null null))
            (`self.SetInventoryItemWidgetStatic` _returnvalue_8 _tempitemdata _render_target_3)))))
    (else
      (`/Game/User_Interfaces/W_Inventory.UpdateInventoryCount` _w_inventory CurrentInventory))))

(fn `RemoveHunger`
  (params (Value :type "Float (double-precision)")))

(fn `SetInventoryItemWidgetAnimated`
  (params (ItemToAdd :type "AnimatedItem Object Reference") (ItemData :type "ItemData Structure") (RenderTarget :type "TextureRenderTarget2D Object Reference"))
  (`Item.SetItemData` ItemToAdd ItemData)
  (`AnimatedItem.SetRenderTarget` ItemToAdd RenderTarget)
  (bind _returnvalue (`|CreateWidget` "/Game/User_Interfaces/w_InventoryItem.w_InventoryItem_C" null ItemData RenderTarget))
  (`/Game/User_Interfaces/W_Inventory.AddItem` (`/Game/User_Interfaces/W_UI.W_Inventory` (`self.W_UI`)) _returnvalue))

(fn `SetInventoryItemWidgetStatic`
  (params (ItemToAdd :type "StaticItem Object Reference") (ItemData :type "ItemData Structure") (RenderTarget :type "TextureRenderTarget2D Object Reference"))
  (bind _w_inventory (`/Game/User_Interfaces/W_UI.W_Inventory` (`self.W_UI`)))
  (`Item.SetItemData` ItemToAdd ItemData)
  (`StaticItem.SetRenderTarget` ItemToAdd RenderTarget)
  (bind _returnvalue (`|CreateWidget` "/Game/User_Interfaces/w_InventoryItem.w_InventoryItem_C" null ItemData RenderTarget))
  (`/Game/User_Interfaces/W_Inventory.AddItem` _w_inventory _returnvalue)
  (`KismetSystemLibrary.PrintText` (`KismetTextLibrary.Conv_IntToText` (`/Game/User_Interfaces/W_Inventory.TotalNumberItems` _w_inventory))))

(fn `TestFunctionItem`
  (params (TestItem :type "Item Object Reference"))
  (`/Engine/EditorBlueprintResources/StandardMacros.IsValid` TestItem
    (:`Is Valid`
      (`KismetSystemLibrary.PrintString` "Is valid item"))
    (:`Is Not Valid`
      (`KismetSystemLibrary.PrintString` "Not Valid"))))

(fn `UserConstructionScript`)